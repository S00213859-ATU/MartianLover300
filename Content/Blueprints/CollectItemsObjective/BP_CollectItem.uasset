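; BP_CollectItem is a spinning jerry can pickup that counts toward a collect-items objective.
; Overlapping its Box enables input on the actor and shows an interact prompt created at BeginPlay; leaving reverses both.
; Pressing Interact decrements CollectablesRemaining on BP_FirstPersonGameMode, adds a collect-item widget to the viewport and destroys the actor.
; The spin is a fixed rotation per tick, so its speed follows frame rate.
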(event `self.ReceiveTick`
  (params (DeltaSeconds :type "Float (single-precision)"))
  ;[1 1 1] To Make it SPIN!!!
  (`SceneComponent.K2_AddWorldRotation` (`self.JerryCan`) (struct :`Yaw` 1.0) false false))

(event `InputAction|Interact`
  (params (Key :type "Key Structure"))
  (:`Pressed`
    ;[1 1 1] Getting all collectables left and taking 1 away from it
    (bind _asbp_first_person_game_mode (cast `/Game/Assets/Characters/FirstPersonArms/Blueprints/BP_FirstPersonGameMode` (`GameplayStatics.GetGameMode`)))
    (bind _result (`/Engine/EditorBlueprintResources/StandardMacros.DecrementInt` (`/Game/Assets/Characters/FirstPersonArms/Blueprints/BP_FirstPersonGameMode.CollectablesRemaining` _asbp_first_person_game_mode))
      (:`  `
        (set `/Game/Assets/Characters/FirstPersonArms/Blueprints/BP_FirstPersonGameMode.CollectablesRemaining` _result _asbp_first_person_game_mode)
        (bind _returnvalue (`|CreateWidget` "/Game/Blueprints/CollectItemsObjective/WP_CollectItemWidget.WP_CollectItemWidget_C"))
        (`UserWidget.AddToViewport` _returnvalue 0)
        (`self.K2_DestroyActor`)))))

(event `self.Box.OnComponentBeginOverlap`
  (params (OverlappedComponent :type "PrimitiveComponent Object Reference") (OtherActor :type "Actor Object Reference") (OtherComp :type "PrimitiveComponent Object Reference") (OtherBodyIndex :type Integer) (bFromSweep :type Boolean) (SweepResult :type "HitResult Structure (by ref)"))
  (`|ExecutionSequence`
    (:`then_0`
      (cast `/Game/Assets/Characters/FirstPersonArms/Blueprints/BP_FirstPersonCharacter` OtherActor)
      ;[1 1 1] If close enough to the box then enable
      (`self.EnableInput` (`GameplayStatics.GetPlayerController` 0)))
    (:`then_1`
      ;[1 1 1] Interact Prompt
      (if (== OtherActor (`GameplayStatics.GetPlayerCharacter` 0))
        (`UserWidget.AddToViewport` (`self.InteractPrompt`) 0)))))

(event `self.Box.OnComponentEndOverlap`
  (params (OverlappedComponent :type "PrimitiveComponent Object Reference") (OtherActor :type "Actor Object Reference") (OtherComp :type "PrimitiveComponent Object Reference") (OtherBodyIndex :type Integer))
  (`|ExecutionSequence`
    (:`then_0`
      (cast `/Game/Assets/Characters/FirstPersonArms/Blueprints/BP_FirstPersonCharacter` OtherActor)
      ;[1 1 1] If not close enough to the box then disable
      (`self.DisableInput` (`GameplayStatics.GetPlayerController` 0)))
    (:`then_1`
      ;[1 1 1] Interact Prompt
      (if (== OtherActor (`GameplayStatics.GetPlayerCharacter` 0))
        (`Widget.RemoveFromParent` (`self.InteractPrompt`))))))

(event `self.ReceiveBeginPlay`
  (bind _returnvalue (`|CreateWidget` "/Game/Blueprints/Prompts/WP_InteractPrompt.WP_InteractPrompt_C"))
  (set `self.InteractPrompt` _returnvalue))

(fn `UserConstructionScript`)