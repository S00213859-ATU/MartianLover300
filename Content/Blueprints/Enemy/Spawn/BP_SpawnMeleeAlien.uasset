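; BP_SpawnMeleeAlien is an enemy spawner actor, set up to repeat spawn waves at its own transform.
; BeginPlay calls SpawnEnemy, which loops over NumberOfEnemies, waits SpawnDelay, then calls itself again with no stop condition.
; The loop body is empty and the SpawnActor node for the Enemy class is disconnected, so the graph spawns nothing as wired.
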(event `self.ReceiveBeginPlay`
  (`self.Spawn Enemy` (`self.Enemy`) (`self.GetTransform`) (`self.Number Of Enemies`)))

(event `Spawn Enemy`
  (params (Enemy :type "Actor Class Reference") (SpawnTransform :type "Transform Structure") (NumberOfEnemies :type Integer))
  (for _ (range NumberOfEnemies)
    _)
  (`KismetSystemLibrary.Delay` (`self.SpawnDelay`))
  (`self.Spawn Enemy` (`self.Enemy`) (`self.GetTransform`) (`self.Number Of Enemies`)))

(fn `UserConstructionScript`)