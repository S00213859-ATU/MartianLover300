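; BP_DronePawn is an AI drone pawn that patrols linked BP_PatrolPoint actors, chases the main character and explodes on contact.
; Patrol loops through each point's NextPoint with a delay, while a detection sphere retargets AIMoveTo to the player and turns the dynamic material red.
; An inner sphere damages the player and triggers Explode, as does depleted health.
; Tick smoothly rotates the drone toward its current goal.
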(event `MoveToGoalTarget`
  (params (NewGoalTarget :type "Actor Object Reference"))
  ;[1 1 1] Move to Goal Target
  (bind _output_get (set `self.GoalActor` NewGoalTarget))
  (`|AIMoveTo` self (0.0 0.0 0.0) _output_get 25.0
    (:`then`
      (`MaterialInstanceDynamic.SetVectorParameterValue` (`self.DynamicDroneMaterial`) "TeamColor" (make `LinearColor` 1.0 0.0 0.0 1.0)))))

(event `self.Sphere.OnComponentBeginOverlap`
  (params (OverlappedComponent :type "PrimitiveComponent Object Reference") (OtherActor :type "Actor Object Reference") (OtherComp :type "PrimitiveComponent Object Reference") (OtherBodyIndex :type Integer) (bFromSweep :type Boolean) (SweepResult :type "HitResult Structure (by ref)"))
  ;[1 1 1] Move to player if sphere overlaps
  (bind _asbp_main_character (cast `/Game/Blueprints/MainCharacter/BP_MainCharacter` OtherActor))
  (`self.MoveToGoalTarget` _asbp_main_character))

(event `self.ExplodeSphere.OnComponentBeginOverlap`
  (params (OverlappedComponent :type "PrimitiveComponent Object Reference") (OtherActor :type "Actor Object Reference") (OtherComp :type "PrimitiveComponent Object Reference") (OtherBodyIndex :type Integer) (bFromSweep :type Boolean) (SweepResult :type "HitResult Structure (by ref)"))
  ;[1 1 1] Move to player and explode when ExplodeSphere overlaps
  (bind _asbp_main_character (cast `/Game/Blueprints/MainCharacter/BP_MainCharacter` OtherActor))
  (`GameplayStatics.ApplyDamage` _asbp_main_character (`self.Damage`))
  (`self.Explode`))

(event `self.ReceiveTick`
  (params (DeltaSeconds :type "Float (single-precision)"))
  (bind _goalactor (`self.GoalActor`))
  ;[1 1 1] Find Actor and rotate to look at them
  (`/Engine/EditorBlueprintResources/StandardMacros.IsValid` _goalactor
    (:`Is Valid`
      (`self.K2_SetActorRotation` (`KismetMathLibrary.RInterpTo` (`self.K2_GetActorRotation`) (`KismetMathLibrary.FindLookAtRotation` (`self.K2_GetActorLocation`) (`self.K2_GetActorLocation` _goalactor)) DeltaSeconds 10.0)))))

(event `self.ReceiveBeginPlay`
  ;[1 1 1] Patrol, move to next Patrol Point
  (add `self.OnTakeAnyDamage` (delegate `OnTakeDamage`))
  (`self.Patrol`))

(event `OnTakeDamage` :!signature `self.OnTakeAnyDamage`
  (params (DamagedActor :type "Actor Object Reference") (Damage :type "Float (single-precision)") (DamageType :type "DamageType Object Reference") (InstigatedBy :type "Controller Object Reference") (DamageCauser :type "Actor Object Reference"))
  ;[1 1 1] Explode at 0 health
  (bind _output_get (set `self.Health` (- (`self.Health`) Damage)))
  (if (<= _output_get 0.0)
    (`self.Explode`)))

(fn `Explode`
  (`GameplayStatics.PlaySoundAtLocation` "/Game/StarterContent/Audio/Explosion_Cue.Explosion_Cue" (`self.K2_GetActorLocation`) (struct) 1.0 1.0 0.0 null null null null)
  (`GameplayStatics.SpawnEmitterAtLocation` "/Game/StarterContent/Particles/P_Explosion.P_Explosion" (`SceneComponent.K2_GetComponentLocation` (`self.Drone_Mesh`)))
  (`self.K2_DestroyActor`))

(fn `UserConstructionScript`
  (bind _returnvalue (`KismetMaterialLibrary.CreateDynamicMaterialInstance` (`PrimitiveComponent.GetMaterial` (`self.Drone_Mesh`) 0)))
  (bind _output_get (set `self.DynamicDroneMaterial` _returnvalue))
  (`PrimitiveComponent.SetMaterial` (`self.Drone_Mesh`) 0 _output_get))