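; BP_CollectItemEscpe is an escape interaction point that wins the game once every collectable has been gathered.
; A box overlap with BP_MainCharacter enables this actor's input on entry and disables it on exit, so Interact only works inside the box.
; On Interact, if the game mode's CollectablesRemaining is zero, it shows WP_WinGameWidget, then after a short delay pauses the game and shows the mouse cursor.
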(event `InputAction|Interact`
  (params (Key :type "Key Structure"))
  (bind _returnvalue (`GameplayStatics.GetPlayerController` 0))
  ;[1 1 1] If there are 0 collectables in the map left
  (:`Pressed`
    (bind _asbp_first_person_game_mode (cast `/Game/Assets/Characters/FirstPersonArms/Blueprints/BP_FirstPersonGameMode` (`GameplayStatics.GetGameMode`)))
    (if (== (`/Game/Assets/Characters/FirstPersonArms/Blueprints/BP_FirstPersonGameMode.CollectablesRemaining` _asbp_first_person_game_mode) 0)
      ;[1 1 1] Then it opens the win game widget
      (bind _returnvalue_2 (`|CreateWidget` "/Game/Blueprints/WinGame/WP_WinGameWidget.WP_WinGameWidget_C" _returnvalue))
      (`UserWidget.AddToViewport` _returnvalue_2 0)
      (`KismetSystemLibrary.Delay` 0.2)
      (`GameplayStatics.SetGamePaused` true)
      (`WidgetBlueprintLibrary.SetInputMode_GameAndUIEx` _returnvalue null)
      (set `PlayerController.bShowMouseCursor` true _returnvalue))))

(event `self.Box.OnComponentBeginOverlap`
  (params (OverlappedComponent :type "PrimitiveComponent Object Reference") (OtherActor :type "Actor Object Reference") (OtherComp :type "PrimitiveComponent Object Reference") (OtherBodyIndex :type Integer) (bFromSweep :type Boolean) (SweepResult :type "HitResult Structure (by ref)"))
  ;[1 1 1] Need to enable and disable inputs when in or our of the box collision
  (cast `/Game/Blueprints/MainCharacter/BP_MainCharacter` OtherActor)
  (`self.EnableInput` (`GameplayStatics.GetPlayerController` 0)))

(event `self.Box.OnComponentEndOverlap`
  (params (OverlappedComponent :type "PrimitiveComponent Object Reference") (OtherActor :type "Actor Object Reference") (OtherComp :type "PrimitiveComponent Object Reference") (OtherBodyIndex :type Integer))
  ;[1 1 1] Need to enable and disable inputs when in or our of the box collision
  (cast `/Game/Blueprints/MainCharacter/BP_MainCharacter` OtherActor)
  (`self.DisableInput` (`GameplayStatics.GetPlayerController` 0)))

(fn `UserConstructionScript`)