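; BP_SpeedBoost is an energy drink pickup that temporarily changes the player's walk speed.
; When a "Player"-tagged actor overlaps its box, it destroys the box and drink components and plays a 2D pickup sound.
; It sets player 0's max walk speed to its MaxWalkSpeed variable, then after Duration resets it to a hard-coded 1000 rather than the previous value.
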(event `self.Box.OnComponentBeginOverlap`
  (params (OverlappedComponent :type "PrimitiveComponent Object Reference") (OtherActor :type "Actor Object Reference") (OtherComp :type "PrimitiveComponent Object Reference") (OtherBodyIndex :type Integer) (bFromSweep :type Boolean) (SweepResult :type "HitResult Structure (by ref)"))
  (bind _charactermovement (`Character.CharacterMovement` (`GameplayStatics.GetPlayerCharacter` 0)))
  ;[1 1 1] Pick Up and Increase Movespeed
  (if (`self.ActorHasTag` OtherActor "Player")
    (`ActorComponent.K2_DestroyComponent` (`self.Box`))
    (`GameplayStatics.PlaySound2D` "/Game/Assets/Sounds/Health/SW_Pickup_Speed2.SW_Pickup_Speed2" 1.0 1.0 0.0 null null)
    (`ActorComponent.K2_DestroyComponent` (`self.EnergyDrink`))
    (set `CharacterMovementComponent.MaxWalkSpeed` (`self.Max Walk Speed`) _charactermovement)
    (`KismetSystemLibrary.Delay` (`self.Duration`))
    (set `CharacterMovementComponent.MaxWalkSpeed` 1000.0 _charactermovement)))

(fn `UserConstructionScript`)