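; Base weapon Blueprint for automatic hitscan guns, handling firing, ammo and reloading.
; StartShooting auto-reloads when empty, then fires and loops FireBullet on a FireRate timer until StopShoting clears it.
; Each shot traces from the muzzle toward a camera-aimed random cone that widens with FiringTime and lower Accuracy, damaging only BP_MainCharacter.
; Shots and reloads broadcast ammo counter updates; reloading has no reserve check, and AimDownSights is empty.
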(event `StartShooting`
  (if (== (`self.Ammo`) 0)
    (`self.Reload`))
  (`self.Fire Bullet`)
  (bind _returnvalue (`KismetSystemLibrary.K2_SetTimer` self "FireBullet" (`self.FireRate`) true))
  (set `self.FiringTimer` _returnvalue))

(event `StopShoting`
  (`KismetSystemLibrary.K2_ClearAndInvalidateTimerHandle` (`self.FiringTimer`))
  (set `self.FiringTime` 0.0))

(event `AimDownSights`)

(fn `CalculateFiringTime`
  (set `self.FiringTime` (+ (`self.FiringTime`) (`GameplayStatics.GetWorldDeltaSeconds`))))

(fn `CanFireWeapon`
  (returns (CanFireWeapon :type Boolean))
  (return (> (`self.Ammo`) 0)))

(fn `Fire Bullet`
  (locals (NewLocalVar :type "HitResult Structure"))
  (bind _returnvalue (`GameplayStatics.GetPlayerCameraManager` 0))
  (if (`self.CanFireWeapon`)
    (`self.CalculateFiringTime`)
    (bind _outhit (`KismetSystemLibrary.LineTraceSingle` (`SceneComponent.GetSocketLocation` (`self.GunMesh`) "Muzzle") (+ (`PlayerCameraManager.GetCameraLocation` _returnvalue) (* (`KismetMathLibrary.RandomUnitVectorInConeInDegrees` (`KismetMathLibrary.GetForwardVector` (`PlayerCameraManager.GetCameraRotation` _returnvalue)) (`KismetMathLibrary.FClamp` (* (`self.FiringTime`) (`KismetMathLibrary.FClamp` (- 1.0 (`self.Accuracy`)) 0.01) 10.0) 0.0 10.0)) (`self.Range`))) "TraceTypeQuery1"))
    (`|ExecutionSequence`
      (:`then_0`
        (bind _output_get (set `self.Ammo` (- (`self.Ammo`) 1)))
        (`self.UpdateAmmoCounter` _output_get (`self.AmmoTotal`)))
      (:`then_1`
        (bind _asbp_main_character (cast `/Game/Blueprints/MainCharacter/BP_MainCharacter` (`.HitActor` (`GameplayStatics.BreakHitResult` _outhit))))
        (`GameplayStatics.ApplyDamage` _asbp_main_character (`self.Damage`))))))

(fn `Reload`
  (bind _clipsize (`self.ClipSize`))
  (if (< (`self.Ammo`) _clipsize)
    (bind _output_get (set `self.AmmoTotal` (- (`self.AmmoTotal`) (- _clipsize (`self.Ammo`)))))
    (bind _output_get_2 (set `self.Ammo` (`self.ClipSize`)))
    (`self.UpdateAmmoCounter` _output_get_2 _output_get)))

(fn `UserConstructionScript`)